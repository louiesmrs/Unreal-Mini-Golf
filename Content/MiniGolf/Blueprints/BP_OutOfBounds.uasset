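; BP_OutOfBounds is a mini golf out-of-bounds actor that returns overlapping pawns to the current ball.
; On BeginPlay it caches the first BP_HoleManager in the level to query for that ball.
; When a pawn overlaps and the ball is valid, the pawn's BallLockComponent teleports and locks it within a fixed radius.
; Player 0's GolfPlayerController then starts looking at the ball.
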(event EventBeginPlay
  (bind _outactors (Actor|GetAllActorsOfClass "/Game/MiniGolf/Blueprints/BP_HoleManager.BP_HoleManager_C"))
  (Variables|Default|SetHoleManagerRef (Utilities|Array|Get(acopy) _outactors)))

(event Collision|EventActorBeginOverlap
  (params (OtherActor :type Actor%20Object%20Reference))
  (bind _holemanagerref (Variables|Default|GetHoleManagerRef))
  (bind _returnvalue (Class|HoleManager|GetCurrentBall _holemanagerref))
  (bind _aspawn (Utilities|Casting|CastToPawn OtherActor))
  (if (Utilities|IsValid _returnvalue)
    (Class|BallLockComponent|TeleportandLocktoBall (Actor|GetComponentbyClass _aspawn "/Script/MiniGolf.BallLockComponent") _returnvalue 1e+02 8e+01 8.0)
    (bind _asgolf_player_controller (Utilities|Casting|CastToGolfPlayerController (Game|GetPlayerController 0)))
    (Class|GolfPlayerController|StartLookatBall _asgolf_player_controller _returnvalue)))

(event EventTick
  (params (DeltaSeconds :type Float%20%28single-precision%29)))

(fn ConstructionScript)